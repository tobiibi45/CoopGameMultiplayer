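; PlayerPawn is a player pawn Blueprint that sets up the HUD for its locally controlled player.
; On BeginPlay it creates crosshair and health indicator widgets and adds both to the viewport.
; Each Tick it prints the HealthComp health value on screen as debug text, also gated by the local-control check.
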(event EventTick
  (params (DeltaSeconds :type Float%20%28single-precision%29))
  (if (Pawn|IsLocallyControlled)
    (Development|PrintString (Utilities|String|ToString(Float) (Variables|/Script/CoopGame.SHealthComponent|GetHealth (Variables|Default|GetHealthComp))) true true "(R=1.000000,G=0.978082,B=0.060304,A=1.000000)" 0.0)))

(event EventBeginPlay
  (if (Pawn|IsLocallyControlled)
    (Utilities|FlowControl|Sequence
      (:then_0
        (bind _returnvalue (UserInterface|CreateWidget "/Game/UI/WBP_CrossHair.WBP_CrossHair_C"))
        (UserInterface|Viewport|AddtoViewport _returnvalue 0))
      (:then_1
        (bind _returnvalue_2 (UserInterface|CreateWidget "/Game/UI/WBP_HealthIndicator.WBP_HealthIndicator_C"))
        (UserInterface|Viewport|AddtoViewport _returnvalue_2 0)))))

(fn ConstructionScript)